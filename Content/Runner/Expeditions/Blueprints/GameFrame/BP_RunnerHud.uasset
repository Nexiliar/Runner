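; BP_RunnerHud is the HUD for a runner game that creates and shows the game's UI widgets.
; On BeginPlay it adds the score widget and, when the game instance flags a first-time play, a tutorial widget with the mouse cursor visible.
; DeadEvent adds the death widget, shows the cursor through the player controller and switches input to UI-only focused on that widget.
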(event `self.ReceiveBeginPlay`
  (bind _returnvalue (`|CreateWidget` "/Game/Runner/UI/W_Scores.W_Scores_C"))
  (`UserWidget.AddToViewport` _returnvalue 0)
  (bind _asbp_game_instance (cast `/Game/Runner/Expeditions/Blueprints/GameFrame/BP_GameInstance` (`GameplayStatics.GetGameInstance`)))
  (if (`/Game/Runner/Expeditions/Blueprints/GameFrame/BP_GameInstance.FirstTime` _asbp_game_instance)
    (bind _returnvalue_2 (`|CreateWidget` "/Game/Runner/UI/W_Tutorial.W_Tutorial_C"))
    (`UserWidget.AddToViewport` _returnvalue_2 0)
    (bind _asbp_player_controller (cast `/Game/Runner/Expeditions/Blueprints/GameFrame/BP_PlayerController` (`self.GetOwningPlayerController`)))
    (set `PlayerController.bShowMouseCursor` true _asbp_player_controller)))

(fn `DeadEvent`
  (bind _returnvalue (`|CreateWidget` "/Game/Runner/UI/W_DeathWidget.W_DeathWidget_C"))
  (`UserWidget.AddToViewport` _returnvalue 0)
  (bind _asbp_player_controller (cast `/Game/Runner/Expeditions/Blueprints/GameFrame/BP_PlayerController` (`self.PlayerOwner`)))
  (set `PlayerController.bShowMouseCursor` true _asbp_player_controller)
  (`WidgetBlueprintLibrary.SetInputMode_UIOnlyEx` _asbp_player_controller _returnvalue))

(fn `UserConstructionScript`)