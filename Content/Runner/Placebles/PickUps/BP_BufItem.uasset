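; BP_BufItem is a runner pickup item that pulses its mesh size as a visual effect.
; BeginPlay derives the pulse limits from the mesh's starting X scale: that size as the minimum and triple it as the maximum.
; Each Tick flips a Forward flag outside those limits, then grows or shrinks the world scale at a frame-rate-scaled linear rate.
; No buff or collection logic is defined in these graphs.
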(event `self.ReceiveBeginPlay`
  (bind _returnvalue_x (`KismetMathLibrary.BreakVector` (`SceneComponent.K2_GetComponentScale` (`self.PickUpMesh`))))
  (`parent.ReceiveBeginPlay`)
  (bind _output_get (set `self.ScaleSize` _returnvalue_x))
  (set `self.MaxScaleSize` (* _output_get 3.0))
  (set `self.MinScaleSize` (/ _output_get 1.0)))

(event `self.ReceiveTick`
  (params (DeltaSeconds :type "Float (single-precision)"))
  (bind _returnvalue (`SceneComponent.K2_GetComponentScale` (`self.PickUpMesh`)))
  (bind _returnvalue_x (`KismetMathLibrary.BreakVector` (`SceneComponent.K2_GetComponentScale` (`self.PickUpMesh`))))
  (`parent.ReceiveTick` DeltaSeconds)
  (set `self.ScaleStep` (* DeltaSeconds 4.0))
  (set `self.ScaleSize` _returnvalue_x)
  (`|ExecutionSequence`
    (:`then_0`
      (if (> (`self.ScaleSize`) (`self.MaxScaleSize`))
        (set `self.bForward` false)
        (elif (< (`self.ScaleSize`) (`self.MinScaleSize`))
          (set `self.bForward` true))))
    (:`then_1`
      (if (`self.bForward`)
        (`SceneComponent.SetWorldScale3D` (`self.PickUpMesh`) (+ _returnvalue (`self.ScaleStep`)))
        (else
          (`SceneComponent.SetWorldScale3D` (`self.PickUpMesh`) (- _returnvalue (`self.ScaleStep`))))))))

(fn `UserConstructionScript`
  (`parent.UserConstructionScript`))