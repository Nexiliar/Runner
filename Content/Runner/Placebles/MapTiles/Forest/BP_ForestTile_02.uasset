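; Forest map tile for a runner game that dresses its sides with scenery and spawns obstacles on it.
; The construction script scatters bush, tree and stone mesh instances at random positions and uniform scales within left and right boxes.
; At BeginPlay it computes points from Left, Mid and Right, spawning random obstacles where a box trace is clear.
; Each spawned obstacle gets its lifetime set from the tile, and a random candidate point is removed.
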(event `self.ReceiveBeginPlay`
  (`parent.ReceiveBeginPlay`)
  (set `self.PointsToSpawn` (`/Game/Runner/Core/BP_Library.ObstacleSpawnLocation` (`self.Left`) (`self.Mid`) (`self.Right`) 800.0 4 300.0))
  (`self.Spawn Obstacle`))

(fn `LocationToSpawn`
  (params (isRight :type Boolean))
  (returns (NewParam :type "Vector Structure"))
  (bind _box (`self.Box`))
  (bind _box1 (`self.Box1`))
  (bind (_returnvalue_x _returnvalue_y) (`KismetMathLibrary.BreakVector` (`KismetMathLibrary.RandomPointInBoundingBox` (`SceneComponent.RelativeLocation` _box1) (`BoxComponent.GetScaledBoxExtent` _box1))))
  (bind (_returnvalue_x_2 _returnvalue_y_2) (`KismetMathLibrary.BreakVector` (`KismetMathLibrary.RandomPointInBoundingBox` (`SceneComponent.RelativeLocation` _box) (`BoxComponent.GetScaledBoxExtent` _box))))
  (if isRight
    (return (`KismetMathLibrary.MakeVector` (+ _returnvalue_x 4502.0) _returnvalue_y))
    (else
      (return (`KismetMathLibrary.MakeVector` (+ _returnvalue_x_2 4502.0) _returnvalue_y_2)))))

(fn `Spawn`
  (params (Amount :type Integer) (Object :type "InstancedStaticMeshComponent Object Reference") (isRightSide :type Boolean))
  (`/Engine/EditorBlueprintResources/StandardMacros.IsValid` Object
    (:`Is Valid`
      (for _ (range (+ Amount 1))
        (`InstancedStaticMeshComponent.AddInstance` Object (`KismetMathLibrary.MakeTransform` (`self.LocationToSpawn` isRightSide) (struct) (`KismetMathLibrary.Conv_DoubleToVector` (`KismetMathLibrary.RandomFloatInRange` 0.4 2.0))))))))

(fn `Spawn Obstacle`
  (bind _obstacles (`self.Obstacles`))
  (for _index (range (`KismetArrayLibrary.Array_Length` (`self.PointsToSpawn`)))
    (bind _output (`|GetArrayItem` (`self.PointsToSpawn`) _index))
    (bind (_outhit _returnvalue) (`KismetSystemLibrary.BoxTraceSingle` :`Start` (+ _output (0.0 0.0 800.0)) :`End` _output :`HalfSize` (1000.0 50.0 50.0) :`TraceChannel` "TraceTypeQuery1" :`DrawTime` 50.0))
    (if (not _returnvalue)
      (bind _returnvalue_2 (`|SpawnActorFromClass` (`|GetArrayItem` _obstacles (`KismetMathLibrary.RandomIntegerInRange` 0 (- (`KismetArrayLibrary.Array_Length` _obstacles) 1))) (`KismetMathLibrary.Conv_VectorToTransform` _output) "Undefined" "OverrideRootScale" null null))
      (bind _asbp_obstacle_base (cast `/Game/Runner/Core/Obstacles/BP_ObstacleBase` _returnvalue_2))
      (`/Game/Runner/Core/Obstacles/BP_ObstacleBase.SetLifeTime` _asbp_obstacle_base self)
      (`KismetArrayLibrary.Array_RemoveItem` (`self.PointsToSpawn`) (`KismetArrayLibrary.Array_Random` (`self.PointsToSpawn`))))))

(fn `UserConstructionScript`
  (bind _tree_04 (`self.Tree_04`))
  (`parent.UserConstructionScript`)
  (`|ExecutionSequence`
    (:`then_0`
      (`self.Spawn` 10 (`self.Bush_01`)))
    (:`then_1`
      (`self.Spawn` 10 (`self.Bush_02`) true))
    (:`then_2`
      (`self.Spawn` 10 (`self.Tree_01`)))
    (:`then_3`
      (`self.Spawn` 10 (`self.Tree_01`) true))
    (:`then_4`
      (`self.Spawn` 10 _tree_04))
    (:`then_5`
      (`self.Spawn` 10 _tree_04 true))
    (:`then_6`
      (`self.Spawn` 10 (`self.Tree_05`)))
    (:`then_7`
      (`self.Spawn` 10 (`self.Tree_07`) true))
    (:`then_8`
      (`self.Spawn` 25 (`self.Stone_01`) true))
    (:`then_9`
      (`self.Spawn` 10 (`self.Stone_02`)))
    (:`then_10`
      (`self.Spawn` 10 null true))
    (:`then_11`
      (`self.Spawn` 10 null true))
    (:`then_12`
      (`self.Spawn` 10 null true))))