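; Forest map tile for a runner game that populates itself with random obstacles when play begins.
; ObstacleSpawnLocation builds candidate points from Left, Mid, Right, Step and AmountOfPoints, then Spawn places a randomly chosen obstacle class at points in that array.
; Each obstacle receives the tile through SetLifeTime, and a random point is removed from the array after each spawn, while the loop is still running.
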(event `self.ReceiveBeginPlay`
  (`parent.ReceiveBeginPlay`)
  (set `self.PointsToSpawn` (`/Game/Runner/Core/BP_Library.ObstacleSpawnLocation` (`self.Left`) (`self.Mid`) (`self.Right`) (`self.Step`) (`self.AmountOfPoints`)))
  (`self.Spawn`))

(event `self.ReceiveTick`
  (params (DeltaSeconds :type "Float (single-precision)")))

(fn `Spawn`
  (bind _obstacles (`self.Obstacles`))
  (for _index (range (`KismetArrayLibrary.Array_Length` (`self.PointsToSpawn`)))
    (bind _returnvalue (`|SpawnActorFromClass` (`|GetArrayItem` _obstacles (`KismetMathLibrary.RandomIntegerInRange` 0 (- (`KismetArrayLibrary.Array_Length` _obstacles) 1))) (`KismetMathLibrary.Conv_VectorToTransform` (`|GetArrayItem` (`self.PointsToSpawn`) _index)) "AdjustIfPossibleButAlwaysSpawn" "OverrideRootScale" null null))
    (bind _asbp_obstacle_base (cast `/Game/Runner/Core/Obstacles/BP_ObstacleBase` _returnvalue))
    (`/Game/Runner/Core/Obstacles/BP_ObstacleBase.SetLifeTime` _asbp_obstacle_base self)
    (`KismetArrayLibrary.Array_RemoveItem` (`self.PointsToSpawn`) (`KismetArrayLibrary.Array_Random` (`self.PointsToSpawn`)))))

(fn `UserConstructionScript`
  (`parent.UserConstructionScript`))