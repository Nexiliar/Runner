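; Forest map tile for the runner game that scatters foliage and spawns obstacles.
; The construction script adds randomly placed, rotated and scaled bush and tree mesh instances inside two side boxes.
; On BeginPlay it builds spawn points from Left, Mid and Right, then spawns random obstacle classes at them, removing a random point after each spawn.
; Each obstacle receives the tile through SetLifeTime.
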(event `self.ReceiveBeginPlay`
  (`parent.ReceiveBeginPlay`)
  (set `self.PointsToSpawn` (`/Game/Runner/Core/BP_Library.ObstacleSpawnLocation` (`self.Left`) (`self.Mid`) (`self.Right`) 1000.0 7))
  (`self.SpawnObstacle`))

(fn `LocationToSpawn`
  (params (isRight :type Boolean) (MinScale :type "Float (double-precision)") (MaxScale :type "Float (double-precision)"))
  (returns (NewParam :type "Vector Structure") (Scale :type "Float (double-precision)"))
  (bind _returnvalue (`KismetMathLibrary.RandomFloatInRange` MinScale MaxScale))
  (bind _box (`self.Box`))
  (bind _box1 (`self.Box1`))
  (bind (_returnvalue_x _returnvalue_y) (`KismetMathLibrary.BreakVector` (`KismetMathLibrary.RandomPointInBoundingBox` (`SceneComponent.RelativeLocation` _box) (`BoxComponent.GetScaledBoxExtent` _box))))
  (bind (_returnvalue_x_2 _returnvalue_y_2) (`KismetMathLibrary.BreakVector` (`KismetMathLibrary.RandomPointInBoundingBox` (`SceneComponent.RelativeLocation` _box1) (`BoxComponent.GetScaledBoxExtent` _box1))))
  (if isRight
    (return (`KismetMathLibrary.MakeVector` (+ _returnvalue_x_2 4502.0) _returnvalue_y_2) _returnvalue)
    (else
      (return (`KismetMathLibrary.MakeVector` (+ _returnvalue_x 4502.0) _returnvalue_y) _returnvalue))))

(fn `Spawn`
  (params (Amount :type Integer) (Object :type "InstancedStaticMeshComponent Object Reference") (isRightSide :type Boolean) (MinScale :type "Float (double-precision)") (MaxScale :type "Float (double-precision)"))
  (bind (_newparam _scale) (`self.LocationToSpawn` isRightSide MinScale MaxScale))
  (`/Engine/EditorBlueprintResources/StandardMacros.IsValid` Object
    (:`Is Valid`
      (for _ (range (+ Amount 1))
        (`InstancedStaticMeshComponent.AddInstance` Object (`KismetMathLibrary.MakeTransform` _newparam (`KismetMathLibrary.MakeRotator` 0.0 0.0 (`KismetMathLibrary.RandomFloatInRange` 0.0 180.0)) (`KismetMathLibrary.Conv_DoubleToVector` _scale)))))))

(fn `SpawnObstacle`
  (bind _obstacles (`self.Obstacles`))
  (for _index (range (`KismetArrayLibrary.Array_Length` (`self.PointsToSpawn`)))
    (bind _returnvalue (`|SpawnActorFromClass` (`|GetArrayItem` _obstacles (`KismetMathLibrary.RandomIntegerInRange` 0 (- (`KismetArrayLibrary.Array_Length` _obstacles) 1))) (`KismetMathLibrary.Conv_VectorToTransform` (`|GetArrayItem` (`self.PointsToSpawn`) _index)) "AdjustIfPossibleButAlwaysSpawn" "OverrideRootScale" null null))
    (bind _asbp_obstacle_base (cast `/Game/Runner/Core/Obstacles/BP_ObstacleBase` _returnvalue))
    (`/Game/Runner/Core/Obstacles/BP_ObstacleBase.SetLifeTime` _asbp_obstacle_base self)
    (`KismetArrayLibrary.Array_RemoveItem` (`self.PointsToSpawn`) (`KismetArrayLibrary.Array_Random` (`self.PointsToSpawn`)))))

(fn `UserConstructionScript`
  (bind _tree_05 (`self.Tree_05`))
  (`parent.UserConstructionScript`)
  (`|ExecutionSequence`
    (:`then_0`
      (`self.Spawn` 30 (`self.Bush_01`) false 0.4 2.0))
    (:`then_1`
      (`self.Spawn` 40 (`self.Bush_02`) true 0.3 1.8))
    (:`then_2`
      (`self.Spawn` 30 (`self.Tree_01`) false 0.3 0.6))
    (:`then_3`
      (`self.Spawn` 30 (`self.Tree_01`) true 0.2 0.8))
    (:`then_4`
      (`self.Spawn` 12 (`self.Tree_03`) false 1.0 2.0))
    (:`then_5`
      (`self.Spawn` 15 (`self.Tree_03`) true 1.0 2.0))
    (:`then_6`
      (`self.Spawn` 40 (`self.Tree_04`) false 0.2 2.0))
    (:`then_7`
      (`self.Spawn` 40 (`self.Tree_04`) true 0.2 1.0))
    (:`then_8`
      (`self.Spawn` 10 _tree_05 false 2.0 8.0))
    (:`then_9`
      (`self.Spawn` 8 _tree_05 true 2.0 12.0))
    (:`then_10`
      (`self.Spawn` 30 (`self.Tree_06`) false 0.6 1.0))
    (:`then_11`
      (`self.Spawn` 20 (`self.Tree_06`) true 0.4 2.5))))