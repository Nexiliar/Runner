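; Forest map tile for the runner that randomizes its quick-time event and obstacles on BeginPlay, and kills the player character on DeathBox overlap.
; A weighted random switch assigns one of three QTE child actors (swing, wall bang or pine bridge) and disables that variant's blocking meshes.
; The choice selects the spawn point set, from which random obstacles spawn and receive the tile through SetLifeTime.
; Scenery Spawn calls in the construction script are disconnected.
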(event `self.ReceiveBeginPlay`
  (`parent.ReceiveBeginPlay`)
  (`self.QTEFunction`))

(event `self.DeathBox.OnComponentBeginOverlap`
  (params (OverlappedComponent :type "PrimitiveComponent Object Reference") (OtherActor :type "Actor Object Reference") (OtherComp :type "PrimitiveComponent Object Reference") (OtherBodyIndex :type Integer) (bFromSweep :type Boolean) (SweepResult :type "HitResult Structure (by ref)"))
  (bind _asbp_third_person_character (cast `/Game/Runner/Core/Characters/BP_ThirdPersonCharacter` OtherActor))
  (`RunnerCharacter.KillChar` _asbp_third_person_character))

(fn `PointsInit`
  (params (isMiddleLaneActive :type Boolean))
  (if isMiddleLaneActive
    (set `self.ObstaclesSpawnPoints` (`|MakeArray` (`self.ObstacleTargetT2`) (`self.ObstacleTargetT3`) (`self.ObstacleTargetT4`) (`self.ObstacleTargetT5`) (`self.ObstacleTargetT6`) (`self.ObstacleTargetT1`) (`self.ObstacleTargetG4`) (`self.ObstacleTargetG5`) (`self.ObstacleTargetG6`) (`self.ObstacleTargetG7`)))
    (else
      (set `self.ObstaclesSpawnPoints` (`|MakeArray` (`self.ObstacleTargetN6`) (`self.ObstacleTargetT2`) (`self.ObstacleTargetT3`) (`self.ObstacleTargetT4`) (`self.ObstacleTargetT5`) (`self.ObstacleTargetT6`) (`self.ObstacleTargetN1`) (`self.ObstacleTargetN2`) (`self.ObstacleTargetN3`) (`self.ObstacleTargetN4`) (`self.ObstacleTargetN5`) (`self.ObstacleTargetT1`) (`self.ObstacleTargetG4`) (`self.ObstacleTargetG5`) (`self.ObstacleTargetG6`) (`self.ObstacleTargetG7`))))))

(fn `QTEFunction`
  (bind _middleplane (`self.MiddlePlane`))
  (bind _firststuck (`self.FirstStuck`))
  (switch `int` (`KismetMathLibrary.RandomIntegerInRange` 0 4)
    (:`Default`
      (`ChildActorComponent.SetChildActorClass` (`self.SecondQTE_Test`) "/Game/Runner/Placebles/Events/BP_QTEMapWallBang.BP_QTEMapWallBang_C" :!label _label)
      (`SceneComponent.SetVisibility` (`self.ThirdQTEPlane`) false false)
      (`SceneComponent.SetVisibility` (`self.SecondStuck`) false false)
      (`PrimitiveComponent.SetCollisionEnabled` (`self.SecondStuck`) "NoCollision")
      (`PrimitiveComponent.SetCollisionEnabled` (`self.ThirdQTEPlane`) "NoCollision")
      (`self.PointsInit` false)
      (`self.SpawnObstacles`))
    (:`0`
      (`ChildActorComponent.SetChildActorClass` (`self.FirstQTE`) "/Game/Runner/Placebles/Events/BP_QTESwingTheWing.BP_QTESwingTheWing_C")
      (`SceneComponent.SetVisibility` _firststuck false false)
      (`SceneComponent.SetVisibility` (`self.FisrtQTEPlane`) false false)
      (`PrimitiveComponent.SetCollisionEnabled` _firststuck "NoCollision")
      (`PrimitiveComponent.SetCollisionEnabled` (`self.FisrtQTEPlane`) "NoCollision")
      (`self.PointsInit` false)
      (`self.SpawnObstacles`))
    (:`1`
      (goto _label))
    (:`2`
      (`ChildActorComponent.SetChildActorClass` (`self.ThirdQTE`) "/Game/Runner/Placebles/Events/BP_QTEMapPineBridge.BP_QTEMapPineBridge_C")
      (`SceneComponent.SetVisibility` _middleplane false false)
      (`PrimitiveComponent.SetCollisionEnabled` _middleplane "NoCollision")
      (`self.PointsInit` true)
      (`self.SpawnObstacles`))))

(fn `SpawnObstacles`
  (bind _obstaclesclass (`self.ObstaclesClass`))
  (bind _obstaclesspawnpoints (`self.ObstaclesSpawnPoints`))
  (bind _returnvalue (`KismetMathLibrary.RandomInteger` (- (`KismetArrayLibrary.Array_Length` _obstaclesspawnpoints) 1)))
  (bind _output (`|GetArrayItem` _obstaclesspawnpoints _returnvalue))
  (for _ (range (+ _returnvalue 1))
    (`KismetArrayLibrary.Array_RemoveItem` (`self.ObstaclesSpawnPoints`) _output)
    (bind _returnvalue_2 (`|SpawnActorFromClass` (`|GetArrayItem` _obstaclesclass (`KismetMathLibrary.RandomInteger` (- (`KismetArrayLibrary.Array_Length` _obstaclesclass) 1))) (`KismetMathLibrary.Conv_VectorToTransform` (`SceneComponent.K2_GetComponentLocation` _output)) "Undefined" "OverrideRootScale" null null))
    (bind _asbp_obstacle_base (cast `/Game/Runner/Core/Obstacles/BP_ObstacleBase` _returnvalue_2))
    (`/Game/Runner/Core/Obstacles/BP_ObstacleBase.SetLifeTime` _asbp_obstacle_base self)))

(fn `UserConstructionScript`
  (`parent.UserConstructionScript`))