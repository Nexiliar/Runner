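; City map tile for the runner that randomizes its surrounding houses and spawns obstacles along Left, Mid and Right lanes.
; The construction script gives each house slot a random mesh and yaw.
; BeginPlay builds lane spawn points, then Spawn box-traces each and places a random obstacle where clear, passing it the tile via SetLifeTime.
; Each successful spawn also removes a random point from the list being iterated, thinning the remaining placements.
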(event `self.ReceiveBeginPlay`
  (`parent.ReceiveBeginPlay`)
  (set `self.PointsToSpawn` (`/Game/Runner/Core/BP_Library.ObstacleSpawnLocation` (`self.Left`) (`self.Mid`) (`self.Right`) (`self.Step`) (`self.AmountOfPoints`) 700.0))
  (`self.Spawn`))

(event `self.ReceiveTick`
  (params (DeltaSeconds :type "Float (single-precision)")))

(fn `EnviromentSpawn`
  (params (Mesh :type "StaticMeshComponent Object Reference"))
  (bind _houses (`self.Houses`))
  (`StaticMeshComponent.SetStaticMesh` Mesh (`|GetArrayItem` _houses (`KismetMathLibrary.RandomIntegerInRange` 0 (- (`KismetArrayLibrary.Array_Length` _houses) 1))))
  (`SceneComponent.K2_SetRelativeRotation` Mesh (`KismetMathLibrary.MakeRotator` 0.0 0.0 (select `int` (`KismetMathLibrary.RandomInteger` 2) :`0` 90.0 :`1` 180.0 :`2` 270.0 :!type "Float (single-precision)")) false false))

(fn `Spawn`
  (bind _obstacles (`self.Obstacles`))
  (for _index (range (`KismetArrayLibrary.Array_Length` (`self.PointsToSpawn`)))
    (bind _output (`|GetArrayItem` (`self.PointsToSpawn`) _index))
    (bind (_outhit _returnvalue) (`KismetSystemLibrary.BoxTraceSingle` :`Start` (+ _output (0.0 0.0 800.0)) :`End` _output :`HalfSize` (1000.0 50.0 50.0) :`TraceChannel` "TraceTypeQuery1" :`DrawTime` 50.0))
    (if (not _returnvalue)
      (bind _returnvalue_2 (`|SpawnActorFromClass` (`|GetArrayItem` _obstacles (`KismetMathLibrary.RandomIntegerInRange` 0 (- (`KismetArrayLibrary.Array_Length` _obstacles) 1))) (`KismetMathLibrary.Conv_VectorToTransform` _output) "Undefined" "OverrideRootScale" null null))
      (bind _asbp_obstacle_base (cast `/Game/Runner/Core/Obstacles/BP_ObstacleBase` _returnvalue_2))
      (`/Game/Runner/Core/Obstacles/BP_ObstacleBase.SetLifeTime` _asbp_obstacle_base self)
      (`KismetArrayLibrary.Array_RemoveItem` (`self.PointsToSpawn`) (`KismetArrayLibrary.Array_Random` (`self.PointsToSpawn`))))))

(fn `UserConstructionScript`
  (`parent.UserConstructionScript`)
  (set `self.PlacedHouses` (`|MakeArray` (`self.Dom_8`) (`self.Dom_2`) (`self.Dom_3`) (`self.Dom_4`) (`self.Dom_5`) (`self.Dom_6`) (`self.Dom_7`) (`self.Dom_1`) (`self.Dom_9`) (`self.Dom_10`) (`self.Dom_11`) (`self.Dom_12`) (`self.Dom_13`) (`self.Dom_14`)))
  (for _array_element (`self.PlacedHouses`)
    (`self.EnviromentSpawn` _array_element)))