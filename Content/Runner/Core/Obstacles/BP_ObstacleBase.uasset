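; Base obstacle for a runner game that gives the player a key-input challenge while inside its trigger box.
; On box entry it starts key capture on BP_ThirdPersonCharacter and shows a WBP_EventControl widget with the desired keys.
; On exit it compares captured keys to DesiredKeys, sets the character's KeysAccept accordingly and removes the widget.
; GenerateKeySequence picks one random arrow key, but its call is disconnected, as is its repeat loop.
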(event `self.ReceiveActorBeginOverlap`
  (params (OtherActor :type "Actor Object Reference")))

(event `self.Box.OnComponentBeginOverlap`
  (params (OverlappedComponent :type "PrimitiveComponent Object Reference") (OtherActor :type "Actor Object Reference") (OtherComp :type "PrimitiveComponent Object Reference") (OtherBodyIndex :type Integer) (bFromSweep :type Boolean) (SweepResult :type "HitResult Structure (by ref)"))
  (bind _asbp_third_person_character (cast `/Game/Runner/Core/Characters/BP_ThirdPersonCharacter` OtherActor))
  (`/Game/Runner/Core/Characters/BP_ThirdPersonCharacter.StartKeysHandle` _asbp_third_person_character)
  (bind _returnvalue (`|CreateWidget` "/Game/Runner/UI/WBP_EventControl.WBP_EventControl_C"))
  (`UserWidget.AddToViewport` _returnvalue 0)
  (`/Engine/EditorBlueprintResources/StandardMacros.IsValid` _returnvalue
    (:`Is Valid`
      (bind _output_get (set `self.EventWidget` _returnvalue))
      (`/Game/Runner/UI/WBP_EventControl.SetDesiredKeys` _output_get (`self.DesiredKeys`)))))

(event `self.Box.OnComponentEndOverlap`
  (params (OverlappedComponent :type "PrimitiveComponent Object Reference") (OtherActor :type "Actor Object Reference") (OtherComp :type "PrimitiveComponent Object Reference") (OtherBodyIndex :type Integer))
  (bind _eventwidget (`self.EventWidget`))
  (bind _asbp_third_person_character (cast `/Game/Runner/Core/Characters/BP_ThirdPersonCharacter` OtherActor))
  (bind _keys (`/Game/Runner/Core/Characters/BP_ThirdPersonCharacter.Stop Keys Handle` _asbp_third_person_character))
  (bind _returnvalue (`KismetArrayLibrary.Array_Identical` _keys (`self.DesiredKeys`)))
  (`KismetSystemLibrary.PrintString` (`KismetStringLibrary.Conv_BoolToString` _returnvalue))
  (if _returnvalue
    (set `/Game/Runner/Core/Characters/BP_ThirdPersonCharacter.KeysAccept` true _asbp_third_person_character)
    (else
      (set `/Game/Runner/Core/Characters/BP_ThirdPersonCharacter.KeysAccept` false _asbp_third_person_character)))
  (`/Engine/EditorBlueprintResources/StandardMacros.IsValid` _eventwidget
    (:`Is Valid`
      (`Widget.RemoveFromParent` _eventwidget))))

(event `self.ObstacleMesh.OnComponentHit`
  (params (HitComponent :type "PrimitiveComponent Object Reference") (OtherActor :type "Actor Object Reference") (OtherComp :type "PrimitiveComponent Object Reference") (NormalImpulse :type "Vector Structure") (Hit :type "HitResult Structure (by ref)")))

(fn `GenerateKeySequence`
  (locals (KeyLeft :type "Key Structure" :default "Left") (RightKey :type "Key Structure" :default "Right") (KeyUp :type "Key Structure" :default "Up") (KeyDown :type "Key Structure" :default "Down"))
  (`KismetArrayLibrary.Array_Clear` (`self.DesiredKeys`))
  (`KismetArrayLibrary.Array_Add` (`self.DesiredKeys`) (select `int` (`KismetMathLibrary.RandomIntegerInRange` 0 3) :`0` (`local.KeyLeft`) :`1` (`local.RightKey`) :`2` (`local.KeyUp`) :`3` (`local.KeyDown`))))

(fn `UserConstructionScript`)