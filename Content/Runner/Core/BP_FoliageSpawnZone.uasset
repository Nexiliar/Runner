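; Editor-time foliage scatter zone that fills a box with instanced meshes from a mesh-to-count map.
; When RunBuild is set, the construction script creates one HISM component per mesh, then clears the flag.
; Line traces from GetTraceParams place randomly scaled instances aligned to surface normals, skipping PM_Foliage hits.
; Attempts per mesh are capped at twice its target count, and BeginPlay does nothing.
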(event `self.ReceiveBeginPlay`)

(fn `UserConstructionScript`
  (locals (SpawnedNumber :type Integer) (Attempts :type Integer))
  (bind (_start _end) (`self.GetTraceParams`))
  (`BoxComponent.SetBoxExtent` (`self.Box`) (`self.BoxExtent`) true)
  (if (`self.RunBuild`)
    (bind _keys (`BlueprintMapLibrary.Map_Keys` (`self.Meshes`)))
    (for _array_element _keys
      (bind (_value _returnvalue) (`BlueprintMapLibrary.Map_Find` (`self.Meshes`) _array_element))
      (if _returnvalue
        (bind _returnvalue_2 (`AddComponent|NODE_AddHierarchicalInstancedStaticMeshComponent-0` :`RelativeTransform` (`self.GetTransform`)))
        (`StaticMeshComponent.SetStaticMesh` _returnvalue_2 _array_element)
        (while (and (< (`local.SpawnedNumber`) _value) (< (`local.Attempts`) (* _value 2)))
          (bind (_outhit _returnvalue_3) (`KismetSystemLibrary.LineTraceSingle` _start _end "TraceTypeQuery1"))
          (`/Engine/EditorBlueprintResources/StandardMacros.IncrementInt` (`local.Attempts`)
            (:`  `
              (if _returnvalue_3
                (if (not (== (`.PhysMat` (`GameplayStatics.BreakHitResult` _outhit)) "/Game/Runner/Core/PM_Foliage.PM_Foliage"))
                  (bind (_returnvalue_roll _returnvalue_pitch _returnvalue_yaw) (`KismetMathLibrary.BreakRotator` (`KismetMathLibrary.Conv_VectorToRotator` (`.Normal` (`GameplayStatics.BreakHitResult` _outhit)))))
                  (`InstancedStaticMeshComponent.AddInstanceWorldSpace` _returnvalue_2 (`KismetMathLibrary.MakeTransform` (`.Location` (`GameplayStatics.BreakHitResult` _outhit)) (`KismetMathLibrary.MakeRotator` _returnvalue_roll (- _returnvalue_pitch 90.0) _returnvalue_yaw) (`KismetMathLibrary.Conv_DoubleToVector` (`KismetMathLibrary.RandomFloatInRange` 0.3 (`self.MaxSizeOfMesh`)))))
                  (`/Engine/EditorBlueprintResources/StandardMacros.IncrementInt` (`local.SpawnedNumber`)))))))
        (set `local.Attempts` 0)
        (set `local.SpawnedNumber` 0)))
    (set `self.RunBuild` false)))