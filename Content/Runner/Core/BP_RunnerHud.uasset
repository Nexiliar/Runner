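; Runner HUD Blueprint that creates the game's start timer, main screen and death widgets.
; BeginPlay shows the start timer, whose end event adds the main screen, shows the cursor, pre-creates event-flow and pause widgets, then calls CallStartGame.
; DeadEvent displays a fresh death widget with UI-only input.
; The pause widget also uses the death widget class, and a first-time tutorial branch is left unconnected.
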(event `self.ReceiveBeginPlay`
  (bind _returnvalue (`|CreateWidget` "/Game/Runner/UI/WBP_StartTimer.WBP_StartTimer_C"))
  (`UserWidget.AddToViewport` _returnvalue 0)
  (add `/Game/Runner/UI/WBP_StartTimer.StartTimerEnd` _returnvalue (delegate `StartSetup`)))

(event `StartSetup`
  (`|ExecutionSequence`
    (:`then_0`
      (bind _returnvalue (`|CreateWidget` "/Game/Runner/UI/WBP_MainScreen.WBP_MainScreen_C"))
      (bind _output_get (set `self.MainWidget` _returnvalue))
      (`UserWidget.AddToViewport` _output_get 0)
      (bind _asbp_player_controller (cast `/Game/Runner/Core/BP_PlayerController` (`self.GetOwningPlayerController`)))
      (set `PlayerController.bShowMouseCursor` true _asbp_player_controller))
    (:`then_1`
      (bind _returnvalue_2 (`|CreateWidget` "/Game/Runner/UI/WBP_EventFlow.WBP_EventFlow_C"))
      (set `self.FlowEvent` _returnvalue_2))
    (:`then_2`
      (bind _returnvalue_3 (`|CreateWidget` "/Game/Runner/UI/WBP_DeathWidget.WBP_DeathWidget_C"))
      (set `self.PauseWidget` _returnvalue_3))
    (:`then_3`
      (`self.StartGame`))))

(fn `DeadEvent`
  (bind _returnvalue (`|CreateWidget` "/Game/Runner/UI/WBP_DeathWidget.WBP_DeathWidget_C"))
  (`UserWidget.AddToViewport` _returnvalue 0)
  (bind _asbp_player_controller (cast `/Game/Runner/Core/BP_PlayerController` (`self.PlayerOwner`)))
  (set `PlayerController.bShowMouseCursor` true _asbp_player_controller)
  (`WidgetBlueprintLibrary.SetInputMode_UIOnlyEx` _asbp_player_controller _returnvalue))

(fn `UserConstructionScript`)