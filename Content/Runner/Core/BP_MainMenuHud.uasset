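; Main menu HUD for the runner game that shows a prologue video on first launch, then the menu.
; On BeginPlay it checks and clears the FirstTime flag on BP_GameInstance, so later loads skip the prologue.
; The first time, it plays the video widget with PrologVideoSound and waits for the widget's end event.
; Both paths create the menu widget, show the cursor and lock input to UI only.
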(event `self.ReceiveBeginPlay`
  (bind _asbp_game_instance (cast `/Game/Runner/Core/BP_GameInstance` (`GameplayStatics.GetGameInstance`)))
  (if (`/Game/Runner/Core/BP_GameInstance.bFirstTime` _asbp_game_instance)
    (set `/Game/Runner/Core/BP_GameInstance.bFirstTime` false _asbp_game_instance)
    (bind _returnvalue (`|CreateWidget` "/Game/Runner/UI/Video/WBP_PrologVideo.WBP_PrologVideo_C"))
    (add `/Game/Runner/UI/Video/WBP_PrologVideo.PrologVideoEnd` _returnvalue (delegate `PrologVideoEnd_Event_0`))
    (`UserWidget.AddToViewport` _returnvalue 0)
    (`SynthComponent.Start` (`self.PrologVideoSound`))
    (else
      (bind _returnvalue_2 (`|CreateWidget` "/Game/Runner/UI/WBP_MenuWidget.WBP_MenuWidget_C" :!label _label))
      (bind _output_get (set `self.MainMenuWidget` _returnvalue_2))
      (`UserWidget.AddToViewport` _output_get 0)
      (bind _asbp_player_controller (cast `/Game/Runner/Core/BP_PlayerController` (`GameplayStatics.GetPlayerController` 0)))
      (set `PlayerController.bShowMouseCursor` true _asbp_player_controller)
      (`WidgetBlueprintLibrary.SetInputMode_UIOnlyEx` _asbp_player_controller _returnvalue_2 "LockAlways"))))

(event `PrologVideoEnd_Event_0`
  (goto _label))

(fn `UserConstructionScript`)