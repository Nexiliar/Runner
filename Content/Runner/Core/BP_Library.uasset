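; BP_Library is a runner-game helper library with one function that builds candidate spawn points for obstacles.
; ObstacleSpawnLocation starts at the world location of each Left, Mid and Right lane component and repeatedly advances along world X.
; Each advance is Step plus StartOffset, so the offset accumulates on every point rather than applying once.
; All three lanes feed a single array through AddUnique, which the function returns.
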(fn `ObstacleSpawnLocation`
  (params (Left :type "SceneComponent Object Reference") (Mid :type "SceneComponent Object Reference") (Right :type "SceneComponent Object Reference") (Step :type "Float (double-precision)") (PointsNum :type Integer) (StartOffset :type "Float (double-precision)"))
  (returns (Locations :type "Array of Vector Structure"))
  (locals (BasicLocationForSpawn :type "Vector Structure") (SpawnPointsArray :type "Array of Vector Structure"))
  (bind _returnvalue (+ (`local.BasicLocationForSpawn`) (`KismetMathLibrary.MakeVector` (+ Step StartOffset))))
  (set `local.BasicLocationForSpawn` (`SceneComponent.K2_GetComponentLocation` Left))
  (for _ (range (+ PointsNum 1))
    (bind _output_get (set `local.BasicLocationForSpawn` _returnvalue))
    (`KismetArrayLibrary.Array_AddUnique` (`local.SpawnPointsArray`) _output_get))
  (set `local.BasicLocationForSpawn` (`SceneComponent.K2_GetComponentLocation` Mid))
  (for _ (range (+ PointsNum 1))
    (bind _output_get_2 (set `local.BasicLocationForSpawn` _returnvalue))
    (`KismetArrayLibrary.Array_AddUnique` (`local.SpawnPointsArray`) _output_get_2))
  (set `local.BasicLocationForSpawn` (`SceneComponent.K2_GetComponentLocation` Right))
  (for _ (range (+ PointsNum 1))
    (bind _output_get_3 (set `local.BasicLocationForSpawn` _returnvalue))
    (`KismetArrayLibrary.Array_AddUnique` (`local.SpawnPointsArray`) _output_get_3))
  (return (`local.SpawnPointsArray`)))