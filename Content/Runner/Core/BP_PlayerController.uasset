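; Player controller for the Runner game that toggles the pause menu with the PauseKey input.
; It gets the pause widget from BP_RunnerHud and tracks the state in its own IsPaused flag.
; Pausing adds the widget to the viewport and pauses the game.
; Unpausing only calls the widget's HideMenu and clears the flag, with no SetGamePaused call in this controller.
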(event `self.ReceiveBeginPlay`)

(event `InputAction|PauseKey` :paused true
  (params (Key :type "Key Structure"))
  (:`Pressed`
    (bind _asbp_runner_hud (cast `/Game/Runner/Core/BP_RunnerHud` (`self.GetHUD`)))
    (set `self.Widget` (`/Game/Runner/Core/BP_RunnerHud.PauseWidget` _asbp_runner_hud))
    (if (`self.bIsPaused`)
      (`/Game/Runner/UI/WBP_DeathWidget.HideMenu` (`self.Widget`))
      (set `self.bIsPaused` false)
      (else
        (`UserWidget.AddToViewport` (`self.Widget`) 0)
        (set `self.bIsPaused` true)
        (`GameplayStatics.SetGamePaused` true)))))

(fn `UserConstructionScript`)